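; Chunreal example actor that demonstrates driving ChucK audio with a global event and reading a ChucK global back into visuals.
; On BeginPlay it sends an inline ChucK sine oscillator script and ID to the audio component and triggers it.
; Pressing Enter broadcasts the global event, which makes the script step and wrap its frequency.
; Tick reads that frequency by ID and maps it to the sphere's scale and material noise.
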(event EventBeginPlay
  (bind _chunreal_audio (Variables|Default|GetChunreal_Audio))
  ;[1 1 1] Write ChucK code as string and compile. Assign ID(string) to ChuckID1
  ; (EM - 06/22/23)
  (Class|AudioParameterControllerInterface|SetStringParameter _chunreal_audio "ChuckCode1" (Utilities|String|MakeLiteralString "// Create a global event and an oscillator 
global Event customEvent; 
SinOsc osc => dac; 
 
100 => global float freq; 
freq => osc.freq; 
 
while (true) 
{ 
    // Wait for customEvent 
    customEvent => now; 
     
    // Increment and wrap frequency 
    (freq + 100)%1000 + 100 => freq; 
    freq => osc.freq; 
}"))
  (Class|AudioParameterControllerInterface|SetStringParameter _chunreal_audio "ChuckID1" (Variables|Default|GetID))
  (Class|AudioParameterControllerInterface|SetTriggerParameter _chunreal_audio "TriggerChuck"))

(event EventTick
  (params (DeltaSeconds :type Float%20%28single-precision%29))
  ;[1 1 1] Get ChucK global variable "freq" using assigned ID and map it to the sphere scale and material noise multiplier
  (bind _returnvalue (Class|ChunrealBlueprint|GetChuckGlobalFloat (Variables|Default|GetID) "freq"))
  (Transformation|SetRelativeScale3D (Variables|Default|GetSphere) (Math|Conversions|ToVector(Float) (Math|Float|MapRangeClamped _returnvalue 1e+02 1e+03 1.0 2.0)))
  (Rendering|Material|SetScalarParameterValueonMaterials (Variables|Default|GetSphere) "Noise" (Math|Float|MapRangeClamped _returnvalue 1e+02 1e+03 0.1 2.0)))

(event Input|KeyboardEvents|Enter
  (params (Key :type Key%20Structure :default "None"))
  ;[1 1 1] Broadcast "customEvent" on Enter
  (:Pressed
    (Class|ChunrealBlueprint|BroadcastChuckGlobalEvent (Variables|Default|GetID) "customEvent")))

(fn ConstructionScript)