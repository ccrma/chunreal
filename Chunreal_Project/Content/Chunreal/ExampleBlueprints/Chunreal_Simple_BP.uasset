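; Example Blueprint for Chunreal that runs ChucK code in Unreal and animates a sphere from the resulting sound's variables.
; BeginPlay passes an inline sine-oscillator sequence and an ID to the audio component as parameters, then triggers it.
; Each Tick reads the ChucK globals by that ID, mapping freq to sphere scale and basefreq to pitch and yaw rotation.
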(event EventBeginPlay
  (bind _chunreal_audio (Variables|Default|GetChunreal_Audio))
  ;[1 1 1] Write ChucK code as string and compile. Assign ID(string) to ChuckID1
  ; (EM - 06/22/23)
  (Class|AudioParameterControllerInterface|SetStringParameter _chunreal_audio "ChuckCode1" (Utilities|String|MakeLiteralString "//Create an oscillator 
SinOsc osc => dac;     
0.75 => osc.gain; 
 
100 => global int basefreq; 
10 => int basefreq_inc; 
0 => global float freq; 
25 => float freq_inc; 
 
while(true) 
{ 
    //Increment and wrap base frequency 
    basefreq + basefreq_inc => basefreq;   
    if(basefreq>200)                       
    { 
	    basefreq/2 => basefreq; 
    } 
         
    basefreq => freq; 
		     
    for(0=>int i; i<8; i++) 
    { 
        //Increment frequency 
        freq + freq_inc => freq;     
        osc.freq(freq); 
        150::ms => now; 
    } 
}"))
  (Class|AudioParameterControllerInterface|SetStringParameter _chunreal_audio "ChuckID1" (Variables|Default|GetID))
  (Class|AudioParameterControllerInterface|SetTriggerParameter _chunreal_audio "TriggerChuck"))

(event EventTick
  (params (DeltaSeconds :type Float%20%28single-precision%29))
  (Utilities|FlowControl|Sequence
    (:then_0
      ;[1 1 1] Get ChucK global variable "freq" using assigned ID and map it to the sphere scale
      (bind _returnvalue (Class|ChunrealBlueprint|GetChuckGlobalFloat (Variables|Default|GetID) "freq"))
      (Transformation|SetRelativeScale3D (Variables|Default|GetSphere) (Math|Conversions|ToVector(Float) (Math|Float|MapRangeClamped _returnvalue 1e+02 4e+02 1.0 2.0))))
    (:then_1
      ;[1 1 1] Get ChucK global variable "basefreq" using assigned ID and map to sphere rotation
      (bind _returnvalue_2 (Class|ChunrealBlueprint|GetChuckGlobalInt (Variables|Default|GetID) "basefreq"))
      (Transformation|SetRelativeRotation (Variables|Default|GetSphere) (Math|Rotator|MakeRotator 0.0 (Math|Float|MapRangeClamped (Math|Conversions|ToFloat(Integer) _returnvalue_2) 1e+02 2e+02 0.0 3.6e+02) (Math|Float|MapRangeClamped (Math|Conversions|ToFloat(Integer) _returnvalue_2) 1e+02 2e+02 0.0 3.6e+02)) false false))))

(fn ConstructionScript)