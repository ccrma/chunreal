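; Chunreal example actor that runs a ChucK chant script through its audio component and links ChucK globals to a sphere's visuals.
; BeginPlay loads chant.ck from disk and triggers it under an ID.
; Each Tick reads the "theFreq" global to drive leaky-integrator smoothed actor rotation and a material exponent.
; Number keys set vibrato depth, which Tick writes back to ChucK and maps to material panner speed.
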(event EventBeginPlay
  (bind _chunreal_audio (Variables|Default|GetChunreal_Audio))
  ;[1 1 1] Read ChucK code from /Content/ChuckFiles/chant.ck  and compile. Assign ID(string) to ChuckID1
  ; (EM - 06/24/23)
  (Class|AudioParameterControllerInterface|SetStringParameter _chunreal_audio "ChuckCode1" (.text (Class|ChunrealBlueprint|ReadFile (Utilities|String|Append (Class|KismetSystemLibrary|GetProjectContentDirectory) "ChuckFiles/" "chant.ck"))))
  (Class|AudioParameterControllerInterface|SetStringParameter _chunreal_audio "ChuckID1" (Variables|Default|GetID))
  (Class|AudioParameterControllerInterface|SetTriggerParameter _chunreal_audio "TriggerChuck"))

(event EventTick
  (params (DeltaSeconds :type Float%20%28single-precision%29))
  (bind _vibratodepth (Variables|Default|GetvibratoDepth))
  (bind _leakagefactor (Variables|Default|GetleakageFactor))
  (bind _leakagefactor_2 (Variables|Default|GetleakageFactor))
  (bind _returnvalue (- 1.0 _leakagefactor))
  (Utilities|FlowControl|Sequence
    (:then_0
      ;[1 1 1] Get ChucK global variable "freq" using assigned ID and map it to sphere rotation (with leaky integrator) and material mask exponent.
      (bind _returnvalue_2 (Class|ChunrealBlueprint|GetChuckGlobalFloat (Variables|Default|GetID) "theFreq"))
      (Rendering|Material|SetScalarParameterValueonMaterials (Variables|Default|GetSphere) "Exponent" (Math|Float|MapRangeClamped _returnvalue_2 7e+01 2e+02 0.75 1.0))
      (Transformation|SetActorRotation (Math|Rotator|MakeRotator (+ (* (.Roll (Math|Rotator|BreakRotator (Variables|Default|Getrotation_previous))) _leakagefactor_2) (* (.Roll (Math|Rotator|BreakRotator (Math|Rotator|MakeRotator 0.0 (Math|Float|MapRangeClamped _returnvalue_2 7e+01 2e+02 0.0 3.6e+02) (Math|Float|MapRangeClamped _returnvalue_2 7e+01 2e+02 0.0 3.6e+02)))) _returnvalue)) (+ (* (.Pitch (Math|Rotator|BreakRotator (Variables|Default|Getrotation_previous))) _leakagefactor_2) (* (.Pitch (Math|Rotator|BreakRotator (Math|Rotator|MakeRotator 0.0 (Math|Float|MapRangeClamped _returnvalue_2 7e+01 2e+02 0.0 3.6e+02) (Math|Float|MapRangeClamped _returnvalue_2 7e+01 2e+02 0.0 3.6e+02)))) _returnvalue)) (+ (* (.Yaw (Math|Rotator|BreakRotator (Variables|Default|Getrotation_previous))) _leakagefactor_2) (* (.Yaw (Math|Rotator|BreakRotator (Math|Rotator|MakeRotator 0.0 (Math|Float|MapRangeClamped _returnvalue_2 7e+01 2e+02 0.0 3.6e+02) (Math|Float|MapRangeClamped _returnvalue_2 7e+01 2e+02 0.0 3.6e+02)))) _returnvalue))))
      (Variables|Default|Setrotation_previous (Math|Rotator|MakeRotator (+ (* (.Roll (Math|Rotator|BreakRotator (Variables|Default|Getrotation_previous))) _leakagefactor_2) (* (.Roll (Math|Rotator|BreakRotator (Math|Rotator|MakeRotator 0.0 (Math|Float|MapRangeClamped _returnvalue_2 7e+01 2e+02 0.0 3.6e+02) (Math|Float|MapRangeClamped _returnvalue_2 7e+01 2e+02 0.0 3.6e+02)))) _returnvalue)) (+ (* (.Pitch (Math|Rotator|BreakRotator (Variables|Default|Getrotation_previous))) _leakagefactor_2) (* (.Pitch (Math|Rotator|BreakRotator (Math|Rotator|MakeRotator 0.0 (Math|Float|MapRangeClamped _returnvalue_2 7e+01 2e+02 0.0 3.6e+02) (Math|Float|MapRangeClamped _returnvalue_2 7e+01 2e+02 0.0 3.6e+02)))) _returnvalue)) (+ (* (.Yaw (Math|Rotator|BreakRotator (Variables|Default|Getrotation_previous))) _leakagefactor_2) (* (.Yaw (Math|Rotator|BreakRotator (Math|Rotator|MakeRotator 0.0 (Math|Float|MapRangeClamped _returnvalue_2 7e+01 2e+02 0.0 3.6e+02) (Math|Float|MapRangeClamped _returnvalue_2 7e+01 2e+02 0.0 3.6e+02)))) _returnvalue)))))
    (:then_2
      ;[1 1 1] Set ChucK global variable "vibratoDepth" and map to the material panner speed
      (Class|ChunrealBlueprint|SetChuckGlobalFloat (Variables|Default|GetID) "vibratoDepth" _vibratodepth)
      (Rendering|Material|SetScalarParameterValueonMaterials (Variables|Default|GetSphere) "Speed" (Math|Float|MapRangeClamped _vibratodepth 0.0001 0.0009 0.1 0.9)))))

(event Input|KeyboardEvents|1
  (params (Key :type Key%20Structure :default "None"))
  ;[1 1 1] Change local vibratoDepth variable by keys
  (:Pressed
    (Variables|Default|SetvibratoDepth 0.0001)))

(event Input|KeyboardEvents|7
  (params (Key :type Key%20Structure :default "None"))
  ;[1 1 1] Change local vibratoDepth variable by keys
  (:Pressed
    (Variables|Default|SetvibratoDepth 0.0007)))

(event Input|KeyboardEvents|8
  (params (Key :type Key%20Structure :default "None"))
  ;[1 1 1] Change local vibratoDepth variable by keys
  (:Pressed
    (Variables|Default|SetvibratoDepth 0.0008)))

(event Input|KeyboardEvents|9
  (params (Key :type Key%20Structure :default "None"))
  ;[1 1 1] Change local vibratoDepth variable by keys
  (:Pressed
    (Variables|Default|SetvibratoDepth 0.0009)))

(event Input|KeyboardEvents|2
  (params (Key :type Key%20Structure :default "None"))
  ;[1 1 1] Change local vibratoDepth variable by keys
  (:Pressed
    (Variables|Default|SetvibratoDepth 0.0002)))

(event Input|KeyboardEvents|3
  (params (Key :type Key%20Structure :default "None"))
  ;[1 1 1] Change local vibratoDepth variable by keys
  (:Pressed
    (Variables|Default|SetvibratoDepth 0.0003)))

(event Input|KeyboardEvents|4
  (params (Key :type Key%20Structure :default "None"))
  ;[1 1 1] Change local vibratoDepth variable by keys
  (:Pressed
    (Variables|Default|SetvibratoDepth 0.0004)))

(event Input|KeyboardEvents|5
  (params (Key :type Key%20Structure :default "None"))
  ;[1 1 1] Change local vibratoDepth variable by keys
  (:Pressed
    (Variables|Default|SetvibratoDepth 0.0005)))

(event Input|KeyboardEvents|6
  (params (Key :type Key%20Structure :default "None"))
  ;[1 1 1] Change local vibratoDepth variable by keys
  (:Pressed
    (Variables|Default|SetvibratoDepth 0.0006)))

(fn ConstructionScript)