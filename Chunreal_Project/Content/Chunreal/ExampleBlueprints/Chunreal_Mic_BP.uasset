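; Example Chunreal actor that passes microphone input through ChucK and makes its mesh react to loudness.
; On BeginPlay it sends inline ChucK code and an ID to the audio component, then triggers it; the code plays the input through and computes windowed FFT-based RMS into a global float.
; Each Tick reads that global by ID and maps it to the mesh's scale, pitch and yaw.
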(event EventBeginPlay
  (bind _chunreal_audio (Variables|Default|GetChunreal_Audio))
  ;[1 1 1] Write ChucK code as string and compile. Assign ID(string) to ChuckID1
  ; (EM - 10/03/23)
  (Class|AudioParameterControllerInterface|SetStringParameter _chunreal_audio "ChuckCode1" (Utilities|String|MakeLiteralString "adc => dac; 
adc => FFT fft =^ RMS rms => blackhole; 
 
// global float for storing rms 
0 => global float rms_val; 
 
// set parameters 
1024 => fft.size; 
// set hann window 
Windowing.hann(1024) => fft.window; 
 
// control loop 
while( true ) 
{ 
    // upchuck: take fft then rms 
    rms.upchuck() @=> UAnaBlob blob; 
    blob.fval(0) => rms_val; 
 
    // advance time 
    fft.size()::samp => now; 
}"))
  (Class|AudioParameterControllerInterface|SetStringParameter _chunreal_audio "ChuckID1" (Variables|Default|GetID))
  (Class|AudioParameterControllerInterface|SetTriggerParameter _chunreal_audio "TriggerChuck"))

(event EventTick
  (params (DeltaSeconds :type Float%20%28single-precision%29))
  (Utilities|FlowControl|Sequence
    (:then_0
      ;[1 1 1] Get ChucK global variable "rms_val" using assigned ID and map it to the sphere scale and rotation
      (bind _returnvalue (Class|ChunrealBlueprint|GetChuckGlobalFloat (Variables|Default|GetID) "rms_val"))
      (Transformation|SetRelativeScale3D (Variables|Default|GetCube) (Math|Conversions|ToVector(Float) (Math|Float|MapRangeClamped _returnvalue 0.0 0.01 1.0 5.0)))
      (Transformation|SetRelativeRotation (Variables|Default|GetCube) (Math|Rotator|MakeRotator 0.0 (Math|Float|MapRangeClamped _returnvalue 0.0 0.01 0.0 3.6e+02) (Math|Float|MapRangeClamped _returnvalue 0.0 0.01 0.0 3.6e+02)) false false))))

(fn ConstructionScript)