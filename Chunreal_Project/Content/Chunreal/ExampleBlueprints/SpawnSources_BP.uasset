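; SpawnSources_BP is a Chunreal example actor that spawns a staggered row of Chunreal_Simple_BP audio sources at runtime.
; On BeginPlay it spawns each source at an offset along Y, gives it a unique ID built from the counter and lowers its ChunrealAudio volume.
; A delayed loop back to the spawn step repeats this every few seconds until the counter reaches its limit.
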(event EventBeginPlay
  (bind _count (Variables|Default|Getcount))
  ;[1 1 1] Spawn ChunrealSimple_BP
  (bind _returnvalue (Game|SpawnActorfromClass "/Game/Chunreal/ExampleBlueprints/Chunreal_Simple_BP.Chunreal_Simple_BP_C" (Math|Transform|MakeTransform (Math|Vector|MakeVectorNetQuantize 0.0 (+ (* _count 300) -6e+02) 1.5e+02) "0, 0, 0" "1.000000,1.000000,1.000000") "Undefined" "MultiplyWithRoot" 0 (Utilities|String|Append "MyChuck" (Utilities|String|ToString(Integer) _count)) 0 :!label _label))
  ;[1 1 1] Set volume multiplier
  (Audio|Components|Audio|SetVolumeMultiplier (Variables|/Game/Chunreal/ExampleBlueprints/Chunreal_Simple_BP.Chunreal_Simple_BP_C|GetChunreal_Audio _returnvalue) 0.25 :!class /Script/Engine.AudioComponent)
  ;[1 1 1] Increment count and trigger spawn again up to 5 times
  (Math|Integer|IncrementInt (Variables|Default|Getcount)
    (:%20%20
      (Utilities|FlowControl|Delay 3.0)
      (if (< (Variables|Default|Getcount) 5)
        (goto _label)))))

(fn ConstructionScript)