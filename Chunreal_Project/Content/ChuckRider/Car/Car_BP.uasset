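; Self-driving grid car that starts driving on BeginPlay and moves forward each Tick at Speed, steered by queued 90-degree turns.
; Left/Right keys set cues that Tick holds until the position along the heading enters a narrow window in each 1000-unit cell.
; Timelines animate each turn, then truncate yaw to a multiple of 90.
; Keys 1/2 drive with rear or seat camera and pawn input disabled; 3 stops and restores the pawn.
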(event Custom|TurnLeft
  (bind _returnvalue (Transformation|GetActorRotation))
  (bind (_roll _pitch _yaw) (Math|Rotator|BreakRotator _returnvalue))
  ;[1 1 1] Turn left
  (Variables|Default|Setrotation_temp (Transformation|GetActorRotation))
  (bind _turn (Timeline|Timeline PlayFromStart)
    (:Update
      (Transformation|SetActorRotation (Math|Rotator|MakeRotator (.Roll (Math|Rotator|BreakRotator (Variables|Default|Getrotation_temp))) (.Pitch (Math|Rotator|BreakRotator (Variables|Default|Getrotation_temp))) (+ (.Yaw (Math|Rotator|BreakRotator (Variables|Default|Getrotation_temp))) (* -9e+01 _turn)))))
    (:Finished
      (Transformation|SetActorRotation (Math|Rotator|MakeRotator _roll _pitch (Math|Conversions|ToFloat(Integer) (* (.ReturnValue (Math|Float|Division(WholeandRemainder) _yaw 9e+01)) 90)))))))

(event Custom|TurnRight
  (bind _returnvalue (Transformation|GetActorRotation))
  (bind (_roll _pitch _yaw) (Math|Rotator|BreakRotator _returnvalue))
  ;[1 1 1] Turn right
  (Variables|Default|Setrotation_temp (Transformation|GetActorRotation))
  (bind _turn (Timeline|TurnRight_timeline PlayFromStart)
    (:Update
      (Transformation|SetActorRotation (Math|Rotator|MakeRotator (.Roll (Math|Rotator|BreakRotator (Variables|Default|Getrotation_temp))) (.Pitch (Math|Rotator|BreakRotator (Variables|Default|Getrotation_temp))) (+ (.Yaw (Math|Rotator|BreakRotator (Variables|Default|Getrotation_temp))) (* 9e+01 _turn)))))
    (:Finished
      (Transformation|SetActorRotation (Math|Rotator|MakeRotator _roll _pitch (Math|Conversions|ToFloat(Integer) (* (.ReturnValue (Math|Float|Division(WholeandRemainder) _yaw 9e+01)) 90)))))))

(event EventBeginPlay
  ;[1 1 1] Switch cameras
  (Variables|Default|Setdriving true)
  (Input|DisableInput (Game|Player|GetPlayerPawn 0) (Game|GetPlayerController 0))
  (Components|Activation|SetActive (Variables|Default|GetCamera_rear) true false)
  (Components|Activation|SetActive (Variables|Default|GetCamera_seat) false false)
  (Game|Player|SetViewTargetwithBlend (Game|GetPlayerController 0) self 1.0 "VTBlend_Linear" 0.0 false))

(event EventTick
  (params (DeltaSeconds :type Float%20%28single-precision%29))
  (bind _returnvalue (Transformation|GetActorForwardVector))
  (bind _returnvalue_2 (Transformation|GetActorLocation))
  (bind _returnvalue_3 (Transformation|GetActorForwardVector))
  (bind _returnvalue_4 (Transformation|GetActorLocation))
  (bind _returnvalue_5 (* _returnvalue _returnvalue_2))
  (bind _returnvalue_6 (* _returnvalue_3 _returnvalue_4))
  (bind _returnvalue_7 (Math|Vector|VectorLength _returnvalue_5))
  (bind _returnvalue_8 (Math|Vector|VectorLength _returnvalue_6))
  (bind _returnvalue_9 (Math|Float|%(Float) _returnvalue_7 1e+03))
  (bind _returnvalue_10 (Math|Float|%(Float) _returnvalue_8 1e+03))
  (Utilities|FlowControl|Sequence
    (:then_0
      ;[1 1 1] Move forward!
      (if (Variables|Default|Getdriving)
        (Transformation|SetActorLocation (+ (Transformation|GetActorLocation) (* (Transformation|GetActorForwardVector) DeltaSeconds (Variables|Default|Getspeed))) false false)))
    (:then_1
      ;[1 1 1] Simple hack to wait for a valid turn
      (if (Variables|Default|GetturnRight_cue)
        (if (and (>= _returnvalue_10 6e+02) (<= _returnvalue_10 625.0))
          (Variables|Default|SetturnRight_cue false)
          (CallFunction|TurnRight))))
    (:then_2
      (if (Variables|Default|GetturnLeft_cue)
        (if (and (>= _returnvalue_9 6e+02) (<= _returnvalue_9 625.0))
          (Variables|Default|SetturnLeft_cue false)
          (CallFunction|TurnLeft))))))

(event Input|KeyboardEvents|1
  (params (Key :type Key%20Structure :default "None"))
  ;[1 1 1] Switch cameras
  (:Pressed
    (Variables|Default|Setdriving true)
    (Input|DisableInput (Game|Player|GetPlayerPawn 0) (Game|GetPlayerController 0))
    (Components|Activation|SetActive (Variables|Default|GetCamera_rear) true false)
    (Components|Activation|SetActive (Variables|Default|GetCamera_seat) false false)
    (Game|Player|SetViewTargetwithBlend (Game|GetPlayerController 0) self 1.0 "VTBlend_Linear" 0.0 false)))

(event Input|KeyboardEvents|2
  (params (Key :type Key%20Structure :default "None"))
  ;[1 1 1] Switch cameras
  (:Pressed
    (Variables|Default|Setdriving true)
    (Input|DisableInput (Game|Player|GetPlayerPawn 0) (Game|GetPlayerController 0))
    (Components|Activation|SetActive (Variables|Default|GetCamera_rear) false false)
    (Components|Activation|SetActive (Variables|Default|GetCamera_seat) true false)
    (Game|Player|SetViewTargetwithBlend (Game|GetPlayerController 0) self 1.0 "VTBlend_Linear" 0.0 false)))

(event Input|KeyboardEvents|3
  (params (Key :type Key%20Structure :default "None"))
  ;[1 1 1] Switch cameras
  (:Pressed
    (Variables|Default|Setdriving false)
    (Input|EnableInput (Game|Player|GetPlayerPawn 0) (Game|GetPlayerController 0))
    (Components|Activation|SetActive (Variables|Default|GetCamera_rear) false false)
    (Components|Activation|SetActive (Variables|Default|GetCamera_seat) false false)
    (Game|Player|SetViewTargetwithBlend (Game|GetPlayerController 0) (Game|Player|GetPlayerPawn 0) 1.0 "VTBlend_Linear" 0.0 false)))

(event Input|KeyboardEvents|Right
  (params (Key :type Key%20Structure :default "None"))
  ;[1 1 1] User inputs
  (:Pressed
    (Variables|Default|SetturnRight_cue true)))

(event Input|KeyboardEvents|Left
  (params (Key :type Key%20Structure :default "None"))
  ;[1 1 1] User inputs
  (:Pressed
    (Variables|Default|SetturnLeft_cue true)))

(fn ConstructionScript)