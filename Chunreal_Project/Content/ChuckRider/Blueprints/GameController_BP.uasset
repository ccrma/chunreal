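; Game controller for ChuckRider that spawns a grid of buildings, with control towers on the border, and makes the city react to audio.
; Submix FFT magnitudes shift through a six-frame history each tick, driving inner building heights row by row as a scrolling spectrum.
; An inline ChucK script, run through ChunrealAudio, computes RMS, which is read back, smoothed and written to the ChuckRider_MPC material parameter collection.
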(event EventBeginPlay
  (bind _chunreal_audio (Variables|Default|GetChunreal_Audio))
  (Utilities|FlowControl|Sequence
    (:then_0
      ;[1 1 1] Initialize buildings
      (CallFunction|SpawnBuildings))
    (:then_1
      ;[1 1 1] Start FFT analysis
      (Class|AudioMixerBlueprintLibrary|StartAnalyzingOutput 0 "Large" "ConstantQ" "Hann" 0.0 "Decibel"))
    (:then_2
      ;[1 1 1] Start RMS analysis via ChuckMain
      (Class|AudioParameterControllerInterface|SetStringParameter _chunreal_audio "ChuckCode1" (Utilities|String|MakeLiteralString "adc => dac; 
adc => FFT fft =^ RMS rms => blackhole; 
 
//global float for storing rms 
0 => global float rms_val; 
 
// set parameters 
1024 => fft.size; 
// set hann window 
Windowing.hann(1024) => fft.window; 
 
// control loop 
while( true ) 
{ 
    // upchuck: take fft then rms 
    rms.upchuck() @=> UAnaBlob blob; 
    blob.fval(0) => rms_val; 
 
    // advance time 
    fft.size()::samp => now; 
}"))
      (Class|AudioParameterControllerInterface|SetStringParameter _chunreal_audio "ChuckID1" "CHUCK_RMS")
      (Class|AudioParameterControllerInterface|SetTriggerParameter _chunreal_audio "TriggerChuck"))))

(event EventTick
  (params (DeltaSeconds :type Float%20%28single-precision%29))
  (Utilities|FlowControl|Sequence
    (:then_0
      ;[1 1 1] Get RMS from ChucK
      (bind _returnvalue (Class|ChunrealBlueprint|GetChuckGlobalFloat "CHUCK_RMS" "rms_val"))
      (Rendering|Material|SetScalarParameterValue "/Game/ChuckRider/Materials/ChuckRider_MPC.ChuckRider_MPC" "rms" (Class|KismetMathLibrary|WeightedMovingAverageFloat _returnvalue (Variables|Default|Getrms_previous) 0.5) :!class /Script/Engine.KismetMaterialLibrary)
      (Variables|Default|Setrms_previous (Class|KismetMathLibrary|WeightedMovingAverageFloat _returnvalue (Variables|Default|Getrms_previous) 0.5)))
    (:then_1
      ;[1 1 1] Get FFT history from master submix
      (bind _magnitudes (Class|AudioMixerBlueprintLibrary|GetMagnitudeforFrequencies (Variables|Default|GetFrequencies) 0))
      (Variables|Default|SetMagnitudes_5 (Variables|Default|GetMagnitudes_4))
      (Variables|Default|SetMagnitudes_4 (Variables|Default|GetMagnitudes_3))
      (Variables|Default|SetMagnitudes_3 (Variables|Default|GetMagnitudes_2))
      (Variables|Default|SetMagnitudes_2 (Variables|Default|GetMagnitudes_1))
      (Variables|Default|SetMagnitudes_1 (Variables|Default|GetMagnitudes_0))
      (Variables|Default|SetMagnitudes_0 _magnitudes))
    (:then_2
      ;[1 1 1] Set buildings height
      (CallFunction|SetBuildingsHeight 1 (Variables|Default|GetMagnitudes_5))
      (CallFunction|SetBuildingsHeight 2 (Variables|Default|GetMagnitudes_4))
      (CallFunction|SetBuildingsHeight 3 (Variables|Default|GetMagnitudes_3))
      (CallFunction|SetBuildingsHeight 4 (Variables|Default|GetMagnitudes_2))
      (CallFunction|SetBuildingsHeight 5 (Variables|Default|GetMagnitudes_1))
      (CallFunction|SetBuildingsHeight 6 (Variables|Default|GetMagnitudes_0)))))

(fn ConstructionScript)

(fn SpawnBuildings
  (bind _grid (Variables|Default|Getgrid))
  (bind _gridseparation (Variables|Default|GetgridSeparation))
  (bind _gridseparation_2 (Variables|Default|GetgridSeparation))
  (bind _returnvalue (- _grid 1))
  (bind _returnvalue_2 (* _grid 0.5 _gridseparation -1.0))
  (bind _returnvalue_3 (* _gridseparation 0.5))
  (bind _returnvalue_4 (+ _returnvalue_2 _returnvalue_3))
  ;[1 1 1] Rows x Columns
  (for _index (range 0 _returnvalue)
    (for _index_2 (range 0 _returnvalue)
      (bind _returnvalue_5 (Game|SpawnActorfromClass "/Game/ChuckRider/Blueprints/Building_BP.Building_BP_C" (Math|Transform|MakeTransform (Math|Vector|MakeVector (+ (* _index _gridseparation_2) _returnvalue_4) (+ (* _index_2 _gridseparation_2) _returnvalue_4) 0.0) "0, 0, 0" (Math|Conversions|ToVector(Float) (Variables|Default|GetbuildingScale))) "Undefined" "MultiplyWithRoot" 0 (Math|Boolean|ORBoolean (== _index_2 0) (== _index_2 _returnvalue) (== _index 0) (== _index _returnvalue)) 5 (* (Math|Random|RandomUnitVector) "1.750000,1.750000,1.750000") 0))
      (Utilities|Array|Add (Variables|Default|GetBuilding_BP) _returnvalue_5))))

(fn SetBuildingsHeight
  (params (row :type Integer) (data :type Array%20of%20Floats%20%28single-precision%29))
  ;[1 1 1] Map FFT magnitudes to inner buildings height
  (for _index (range 1 (- (Variables|Default|Getgrid) 2))
    (Default|SetHeight (Utilities|Array|Get(acopy) (Variables|Default|GetBuilding_BP) (+ _index (* (Variables|Default|Getgrid) row))) (* (Variables|Default|GetbuildingScale) (Math|Float|MapRangeClamped (Utilities|Array|Get(acopy) data (- _index 1)) 0.0 1e+01 0.5 1.0)))))