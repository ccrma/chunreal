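; Generative music actor that plays three procedural ChucK layers: bass, filtered noise and delayed percussion.
; On BeginPlay it sends inline ChucK code to three ChuckSub audio components and triggers each one.
; Each script waits on a global myClock event, not broadcast here, to stay in sync.
; The FadeIn timeline then drives per-layer global volume floats on "ChuckParent", raising the layers from silence.
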(event EventBeginPlay
  (bind _chucksub1 (Variables|Default|GetChuckSub1))
  (bind _chucksub2 (Variables|Default|GetChuckSub2))
  (bind _chucksub3 (Variables|Default|GetChuckSub3))
  (Utilities|FlowControl|Sequence
    (:then_0
      ;[1 1 1] Layers of ChucK scripts...
      (Class|AudioParameterControllerInterface|SetStringParameter _chucksub1 "ChuckCode1" (Utilities|String|MakeLiteralString "// global event 
global Event myClock; 
 
0.0 => global float BASS_VOLUME; 
 
// patch 
Blit s => ADSR adsr => JCRev r => dac; 
adsr.set( 5::ms, 0::ms, 1.0, 250::ms ); 
.1 => r.mix; 
 
// an array 
[ 2, 2, 2, 2, 2, 3 ] @=> int hi[]; 
 
// infinite time loop 
while( true ) 
{    
     BASS_VOLUME => s.gain; 
 
     //Wait for global clock 
    myClock => now; 
 
    // frequency 
    Std.mtof( 24 + hi[Math.random2(0,hi.size()-1)] ) => s.freq; 
 
    // harmonics 
    Math.random2( 5, 10 ) => s.harmonics; 
 
    adsr.keyOn(); 
    10::ms => now; 
    adsr.keyOff(); 
}"))
      (Class|AudioParameterControllerInterface|SetTriggerParameter _chucksub1 "TriggerChuck")
      (Class|AudioParameterControllerInterface|SetStringParameter _chucksub2 "ChuckCode1" (Utilities|String|MakeLiteralString "// global event 
global Event myClock; 
 
0.0 => global float NOISE_VOLUME; 
 
Noise n => LPF lpf => JCRev r => dac; 
5.0 => lpf.Q; 
0.2 => r.mix; 
 
while (true) 
{ 
    NOISE_VOLUME => n.gain; 
 
    // Wait for global clock 
    myClock => now; 
 
    Math.random2f( 50.0, 1000.0 ) => lpf.freq; 
}"))
      (Class|AudioParameterControllerInterface|SetTriggerParameter _chucksub2 "TriggerChuck")
      (Class|AudioParameterControllerInterface|SetStringParameter _chucksub3 "ChuckCode1" (Utilities|String|MakeLiteralString "// global event 
global Event myClock; 
 
0.0 => global float PERC_VOLUME; 
 
Blit s => ADSR adsr => Gain g => JCRev r => dac; 
g => Gain feedback => DelayL delay => g; 
 
adsr.set( 1::ms, 0::ms, 1.0, 1::ms ); 
10000::ms => delay.max; 
125::ms => delay.delay; 
0.5 => feedback.gain; 
.05 => r.mix; 
 
// infinite time loop 
while( true ) 
{    
     PERC_VOLUME => s.gain; 
 
     //Wait for global clock 
    myClock => now; 
 
    // frequency 
    Std.mtof( 86 ) => s.freq; 
 
    // harmonics 
    Math.random2( 5, 10 ) => s.harmonics; 
 
    adsr.keyOn(); 
    1::ms => now; 
    adsr.keyOff(); 
}"))
      (Class|AudioParameterControllerInterface|SetTriggerParameter _chucksub3 "TriggerChuck"))
    (:then_1
      ;[1 1 1] Fade in volume by setting global float variables
      (bind (_direction _bass _noise _perc) (Timeline|FadeIn Play)
        (:Update
          (Class|ChunrealBlueprint|SetChuckGlobalFloat "ChuckParent" "BASS_VOLUME" _bass)
          (Class|ChunrealBlueprint|SetChuckGlobalFloat "ChuckParent" "NOISE_VOLUME" _noise)
          (Class|ChunrealBlueprint|SetChuckGlobalFloat "ChuckParent" "PERC_VOLUME" _perc))))))

(event EventTick
  (params (DeltaSeconds :type Float%20%28single-precision%29)))

(fn ConstructionScript)