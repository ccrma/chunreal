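; Building actor for ChuckRider that assembles itself from stacked, attached block actors, one per story.
; BeginPlay spawns the blocks, flags the first and passes on light settings and the control tower flag.
; Control tower buildings also send inline ChucK code to ChuckMain, playing a chorused sine oscillator with randomized pitch and modulation.
; SetHeight stretches the building's relative Z scale, smoothed by a weighted moving average.
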(event EventBeginPlay
  (bind _chuckmain (Variables|Default|GetChuckMain))
  (Utilities|FlowControl|Sequence
    (:then_0
      ;[1 1 1] Initialize building blocks
      (for _index (range 0 (- (Variables|Default|Getstory) 1))
        (bind _returnvalue (Game|SpawnActorfromClass "/Game/ChuckRider/Blueprints/BuildingBlock_BP.BuildingBlock_BP_C" (Math|Transform|MakeTransform (Math|Vector|MakeVector 0.0 0.0 (Math|Conversions|ToFloat(Integer) (* _index 100))) "0, 0, 0" "1.000000,1.000000,1.000000") "Undefined" "MultiplyWithRoot" 0 (== _index 0) (Variables|Default|GetcontrolTower) (Variables|Default|GetlightScale) 0.2 0))
        (Transformation|AttachActorToActor _returnvalue self "None" "KeepRelative" "KeepRelative" "KeepRelative" true)))
    (:then_1
      ;[1 1 1] Random oscillator per building
      (if (Variables|Default|GetcontrolTower)
        (Class|AudioParameterControllerInterface|SetStringParameter _chuckmain "ChuckCode1" (Utilities|String|MakeLiteralString "SinOsc osc => Chorus chorus => dac; 
0.1 => osc.gain; 
Math.random2f( 50.0, 1000.0 ) => osc.freq; 
Math.random2f( 0.01, 0.05 ) => chorus.modFreq; 
Math.random2f( 0.0, 1.0 ) => chorus.modDepth; 
 
while( true ) 
{ 
   1000::ms => now; 
}"))
        (Class|AudioParameterControllerInterface|SetTriggerParameter _chuckmain "TriggerChuck")))))

(fn ConstructionScript)

(fn SetHeight
  (params (height :type Float%20%28double-precision%29))
  (bind _returnvalue (Class|Actor|GetActorRelativeScale3D))
  ;[1 1 1] Stretch building relative height
  (Transformation|SetActorRelativeScale3D (Math|Vector|MakeVector (.x _returnvalue) (.y _returnvalue) (Class|KismetMathLibrary|WeightedMovingAverageFloat height (Variables|Default|Getheight_previous) 0.05)))
  (Variables|Default|Setheight_previous (Class|KismetMathLibrary|WeightedMovingAverageFloat height (Variables|Default|Getheight_previous) 0.05)))