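; BuildingBlock_BP is a building segment that decorates its four side faces with randomly placed lights.
; The construction script keeps road light spheres only on the first-floor block and the wireframe only on the control tower, destroying them otherwise.
; On BeginPlay, SpawnLights rolls LightProbability for each cell of a 4x4 grid per face, spawning scaled Light_BP actors attached to the block, rotated for the second pair of faces.
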(event EventBeginPlay
  (CallFunction|SpawnLights (Variables|Default|GetLight%20Scale)))

(fn ConstructionScript
  (Utilities|FlowControl|Sequence
    (:then_0
      ;[1 1 1] Only the first floor block has road lights!
      (if (not (Variables|Default|GetfirstBlock))
        (Components|DestroyComponent (Variables|Default|GetSphere1))))
    (:then_1
      ;[1 1 1] Only the "control tower" has wireframe
      (if (not (Variables|Default|GetcontrolTower))
        (Components|DestroyComponent (Variables|Default|GetWireframe))))))

(fn SpawnLights
  (params (lightScale :type Vector :default "1.000000,1.000000,1.000000"))
  ;[1 1 1] Spawn light blocks in 3D grids
  (LocalVariables|SetlightScale_local lightScale)
  (Utilities|FlowControl|Sequence
    (:then_0
      (for _index (range 0 1)
        (for _index_2 (range 0 3)
          (for _index_3 (range 0 3)
            (if (< (Math|Random|RandomFloat) (Variables|Default|Getlight_probability))
              (bind _returnvalue (Game|SpawnActorfromClass "/Game/ChuckRider/Blueprints/Light_BP.Light_BP_C" (Math|Transform|MakeTransform (Math|Vector|MakeVector (Math|Conversions|ToFloat(Integer) (+ (* (- 1 _index) -100) 50)) (- (Math|Float|MakeLiteralFloat 3e+01) (* _index_2 20)) (- (Math|Float|MakeLiteralFloat 8e+01) (* _index_3 20))) "0, 0, 0" (LocalVariables|GetlightScale_local)) "Undefined" "MultiplyWithRoot" 0 0))
              (Transformation|AttachActorToActor _returnvalue self "None" "KeepRelative" "KeepRelative" "KeepRelative" true))))))
    (:then_1
      (for _index_4 (range 0 1)
        (for _index_5 (range 0 3)
          (for _index_6 (range 0 3)
            (if (< (Math|Random|RandomFloat) (Variables|Default|Getlight_probability))
              (bind _returnvalue_2 (Game|SpawnActorfromClass "/Game/ChuckRider/Blueprints/Light_BP.Light_BP_C" (Math|Transform|MakeTransform (Math|Vector|MakeVector (- (Math|Float|MakeLiteralFloat 3e+01) (* _index_5 20)) (Math|Conversions|ToFloat(Integer) (+ (* (- 1 _index_4) -100) 50)) (- (Math|Float|MakeLiteralFloat 8e+01) (* _index_6 20))) "0.000000,90.000000,0.000000" (LocalVariables|GetlightScale_local)) "Undefined" "MultiplyWithRoot" 0 0))
              (Transformation|AttachActorToActor _returnvalue_2 self "None" "KeepRelative" "KeepRelative" "KeepRelative" true))))))))